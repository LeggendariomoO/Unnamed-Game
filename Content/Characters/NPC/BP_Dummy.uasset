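; Melee enemy NPC that chases and attacks the player once it spots them, with its health held in a dummy health component.
; PawnSensing starts the chase; sighting or damage widens its vision to a 180-degree peripheral angle.
; Reaching the player plays an attack montage and arms a damage sphere that disarms after hitting the player.
; While alive, damage triggers random hit sounds and montages, knockback along the player's facing, and health loss.
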(event OnSeePawn(PawnSensing)
  (params (Pawn :type Pawn%20Object%20Reference))
  (if (Variables|Default|GetAlive)
    (if (Variables|Default|GetIsSeeing)
      _
      (else
        (Development|PrintText "Ti ho visto!")
        (bind _output_get (Variables|Default|SetIsSeeing true))))
    (Class|PawnSensingComponent|SetPeripheralVisionAngle (Variables|Default|GetPawnSensing) 1.8e+02)
    (if _output_get
      (CallFunction|MovetoPlayer))))

(event OnComponentBeginOverlap(DamageSphere)
  (params (OverlappedComponent :type Primitive%20Component%20Object%20Reference) (OtherActor :type Actor%20Object%20Reference) (OtherComp :type Primitive%20Component%20Object%20Reference) (OtherBodyIndex :type Integer) (bFromSweep :type Boolean) (SweepResult :type Hit%20Result%20Structure%20%28by%20ref%29))
  (bind _asbp_player_character (Utilities|Casting|CastToBP_PlayerCharacter OtherActor))
  (Variables|Default|SetAs%20BP%20Player%20Character _asbp_player_character)
  (Default|ChangeHealth (Variables|/Game/FirstPerson/Blueprints/BP_PlayerCharacter.BP_PlayerCharacter_C|GetBPC_PlayerStats (Variables|Default|GetAs%20BP%20Player%20Character)) -5.0)
  (Variables|/Script/Engine.PrimitiveComponent|SetbGenerateOverlapEvents (Variables|Default|GetDamageSphere) false))

(event Custom|MoveToPlayer
  (AI|AIMoveTo self "0, 0, 0" (stale EventBeginPlay _output_get) 7e+01 true
    (:OnSuccess
      (if (Variables|Default|GetCanAttack)
        (Utilities|FlowControl|Delay 0.6)
        (Variables|Default|SetCanAttack false)
        (bind _returnvalue (Animation|PlayAnimMontage "/Game/Characters/Mannequins/Anims/Unarmed/Attack/MM_Attack_01_Montage.MM_Attack_01_Montage" 1.0 "None"))
        (Variables|/Script/Engine.PrimitiveComponent|SetbGenerateOverlapEvents (Variables|Default|GetDamageSphere) true)
        (Utilities|FlowControl|Delay _returnvalue)
        (Variables|Default|SetCanAttack true)))))

(event EventBeginPlay
  (bind _asbp_player_character (Utilities|Casting|CastToBP_PlayerCharacter (Game|Player|GetPlayerPawn 0)))
  (bind _output_get (Variables|Default|SetAs%20BP%20Player%20Character _asbp_player_character)))

(event Game|Damage|EventAnyDamage
  (params (Damage :type Float%20%28single-precision%29) (DamageType :type Damage%20Type%20Object%20Reference) (InstigatedBy :type Controller%20Object%20Reference) (DamageCauser :type Actor%20Object%20Reference))
  (Variables|Default|SetIsSeeing true)
  (Class|PawnSensingComponent|SetPeripheralVisionAngle (Variables|Default|GetPawnSensing) 1.8e+02)
  (if (Variables|Default|GetAlive)
    (Audio|PlaySoundatLocation (Utilities|Array|Get(acopy) (Variables|Default|GetHitSounds) (Math|Random|RandomIntegerinRange 0 (- (Utilities|Array|Length (Variables|Default|GetHitSounds)) 1))) (Transformation|GetWorldLocation (Variables|Character|GetMesh)) "0, 0, 0" 1.0 1.0 0.0 0 0 0 0)
    (Animation|PlayAnimMontage (Utilities|Array|Get(acopy) (Variables|Default|GetHitAnimation) (Math|Random|RandomIntegerinRange 0 (- (Utilities|Array|Length (Variables|Default|GetHitAnimation)) 1))) 1.0 "None")
    (bind _asbp_player_character (Utilities|Casting|CastToBP_PlayerCharacter (Game|GetPlayerCharacter 0)))
    (Character|LaunchCharacter (* (Math|Vector|GetForwardVector (Transformation|GetActorRotation _asbp_player_character)) 7e+02) false false)
    (Default|ChangeHealth (Variables|Default|GetBP_DummyHealt) (* Damage -1.0))))

(fn ConstructionScript
  (bind _bp_dummyhealt (Variables|Default|GetBP_DummyHealt))
  (bind _output_get (Variables|/Game/Characters/NPC/BP_DummyHealt.BP_DummyHealt_C|SetMaxHealth _bp_dummyhealt 4e+01))
  (Variables|/Game/Characters/NPC/BP_DummyHealt.BP_DummyHealt_C|SetCurrentHealth _bp_dummyhealt _output_get))