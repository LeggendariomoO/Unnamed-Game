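; Health component for Morigesh-based characters that tracks health and handles their death.
; ChangeHealth adds a signed amount while health is positive, caps it at the maximum, and calls KillDummy at zero or below.
; KillDummy casts the owner, plays the death montage, switches the mesh to ragdoll shortly before it ends, then destroys the actor after delays.
; The child-class variant also hides its mesh and destroys a MagicBarrier actor.
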(event Custom|KillDummy
  (bind _returnvalue (Components|GetOwner))
  (Development|PrintText "Morto")
  (bind _asbp_morigesh_player_character_child (Utilities|Casting|CastToBP_MorigeshPlayerCharacter_Child _returnvalue)
    (:then
      (Variables|Default|SetAlive false)
      (bind _returnvalue_2 (Animation|PlayAnimMontage _asbp_morigesh_player_character_child "/Game/Characters/Animations/AI/Death_Montage.Death_Montage" 1.0 "None"))
      (Utilities|FlowControl|Delay (- _returnvalue_2 0.25))
      (Physics|SetSimulatePhysics (Variables|/Script/Engine.Character|GetMesh _asbp_morigesh_player_character_child) true)
      (Utilities|FlowControl|Delay 5.0)
      (bind _asbp_morigesh_player_character_child_2 (Utilities|Casting|CastToBP_MorigeshPlayerCharacter_Child (Components|GetOwner)))
      (Rendering|SetVisibility (Variables|/Script/Engine.Character|GetMesh _asbp_morigesh_player_character_child_2) false false)
      (Utilities|FlowControl|Delay 2.0)
      (Actor|DestroyActor (Variables|Default|GetMagic%20Barrier))
      (Actor|DestroyActor _asbp_morigesh_player_character_child))
    (:CastFailed
      (bind _asbp_morigesh_player_character (Utilities|Casting|CastToBP_MorigeshPlayerCharacter _returnvalue))
      (Variables|Default|SetAlive false)
      (bind _returnvalue_3 (Animation|PlayAnimMontage _asbp_morigesh_player_character "/Game/Characters/Animations/AI/Death_Montage.Death_Montage" 1.0 "None"))
      (Utilities|FlowControl|Delay (- _returnvalue_3 0.25))
      (Physics|SetSimulatePhysics (Variables|/Script/Engine.Character|GetMesh _asbp_morigesh_player_character) true)
      (Utilities|FlowControl|Delay 5.0)
      (Actor|DestroyActor _asbp_morigesh_player_character))))

(event EventBeginPlay
  (bind _output_get (Variables|Default|SetMaxHealth (Variables|Default|GetMaxHealth)))
  (Variables|Default|SetCurrentHealth _output_get))

(event EventTick
  (params (DeltaSeconds :type Float%20%28single-precision%29)))

(fn ChangeHealth
  (params (Changing :type Float%20%28double-precision%29))
  (if (> (Variables|Default|GetCurrentHealth) 0.0)
    (bind _output_get (Variables|Default|SetCurrentHealth (+ Changing (Variables|Default|GetCurrentHealth))))
    (if (<= _output_get 0.0)
      (Variables|Default|SetAlive false)
      (CallFunction|KillDummy)
      (elif (>= _output_get (Variables|Default|GetMaxHealth))
        (bind _output_get_2 (Variables|Default|SetCurrentHealth (Variables|Default|GetMaxHealth)))
        (Development|PrintText (Utilities|Text|ToText(Float) _output_get_2 "HalfToEven"))))))