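; Health component for the BP_Dummy NPC that tracks hit points and handles the dummy's death.
; ChangeHealth applies a signed delta while health is above zero, capping it at the maximum and calling KillDummy when it runs out.
; KillDummy clears the owner's Alive flag, plays a random death montage, switches the mesh to ragdoll physics just before it ends, then destroys the actor after a delay.
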(event Custom|KillDummy
  (Development|PrintText "Morto")
  (bind _asbp_dummy (Utilities|Casting|CastToBP_Dummy (Components|GetOwner)))
  (Variables|/Game/Characters/NPC/BP_Dummy.BP_Dummy_C|SetAlive _asbp_dummy false)
  (bind _returnvalue (Animation|PlayAnimMontage _asbp_dummy (Utilities|Array|Get(acopy) (Variables|Default|GetDeathAnimations) (Math|Random|RandomIntegerinRange 0 (- (Utilities|Array|Length (Variables|Default|GetDeathAnimations)) 1))) 1.0 "None"))
  (Utilities|FlowControl|Delay (- _returnvalue 0.25))
  (Physics|SetSimulatePhysics (Variables|/Script/Engine.Character|GetMesh _asbp_dummy) true)
  (Utilities|FlowControl|Delay 5.0)
  (Actor|DestroyActor _asbp_dummy))

(event EventBeginPlay
  (Variables|Default|SetMaxHealth 1e+02)
  (Variables|Default|SetCurrentHealth 1e+02))

(event EventTick
  (params (DeltaSeconds :type Float%20%28single-precision%29)))

(fn ChangeHealth
  (params (Changing :type Float%20%28double-precision%29))
  (if (> (Variables|Default|GetCurrentHealth) 0.0)
    (bind _output_get (Variables|Default|SetCurrentHealth (+ Changing (Variables|Default|GetCurrentHealth))))
    (if (<= _output_get 0.0)
      (CallFunction|KillDummy)
      (elif (>= _output_get (Variables|Default|GetMaxHealth))
        (bind _output_get_2 (Variables|Default|SetCurrentHealth (Variables|Default|GetMaxHealth)))
        (Development|PrintText (Utilities|Text|ToText(Float) _output_get_2 "HalfToEven"))))))